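; BP_BullRunGameState builds the road track for a bull run game when play begins.
; BeginPlay spawns runs of straight BP_Road tiles separated by two turn tiles, each randomly chosen as BP_LeftRoad or BP_RightRoad.
; Each spawned tile's attach transform becomes NextSpawnPoint, so tiles chain end to end into a track generated once at startup.
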(event `self.ReceiveBeginPlay`
  (for _ (range 13)
    (`self.AddRoadTile`))
  (`self.AddTurningRoadTile`)
  (for _ (range 7)
    (`self.AddRoadTile`))
  (`self.AddTurningRoadTile`)
  (for _ (range 7)
    (`self.AddRoadTile`)))

(fn `AddRoadTile`
  (bind _returnvalue (`|SpawnActorFromClass` "/Game/Blueprints/BP_Road.BP_Road_C" (`self.NextSpawnPoint`) "Undefined" "OverrideRootScale" null null))
  (bind _transform (`/Game/Blueprints/BP_Road.GetAttachTransform` _returnvalue))
  (set `self.NextSpawnPoint` _transform)
  (return))

(fn `AddTurningRoadTile`
  (if (<= (`KismetMathLibrary.RandomIntegerInRange` 0 1) 0)
    (bind _returnvalue (`|SpawnActorFromClass` "/Game/Blueprints/BP_LeftRoad.BP_LeftRoad_C" (`self.NextSpawnPoint`) "Undefined" "OverrideRootScale" null null))
    (bind _transform (`/Game/Blueprints/BP_LeftRoad.GetAttachTransform` _returnvalue))
    (set `self.NextSpawnPoint` _transform)
    (else
      (bind _returnvalue_2 (`|SpawnActorFromClass` "/Game/Blueprints/BP_RightRoad.BP_RightRoad_C" (`self.NextSpawnPoint`) "Undefined" "OverrideRootScale" null null))
      (bind _transform_2 (`/Game/Blueprints/BP_RightRoad.GetAttachTransform` _returnvalue_2))
      (set `self.NextSpawnPoint` _transform_2)))
  (return))

(fn `UserConstructionScript`)